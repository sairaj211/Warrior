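; Base projectile actor that handles the sound and visual effects of a projectile's launch, flight and impact.
; On BeginPlay it plays a spawn sound, attaches a flying sound to the root and spawns a muzzle effect oriented along its forward vector.
; A separate OnSpawnProjectileHitFX event plays the impact sound and effect at a given hit location.
; Each asset is validity-checked first, and the graph contains no movement, collision or damage logic.
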(event `self.ReceiveBeginPlay`
  (`|ExecutionSequence`
    (:`then_0`
      (bind _projectilespawnsound (`self.ProjectileSpawnSound`)
        (:`then`
          (`GameplayStatics.PlaySoundAtLocation` _projectilespawnsound (`self.K2_GetActorLocation`) (struct) 1.0 1.0 0.0 null null null null))
        (:`else`)))
    (:`then_1`
      (bind _projectileflyingsound (`self.ProjectileFlyingSound`)
        (:`then`
          (`GameplayStatics.SpawnSoundAttached` _projectileflyingsound (`self.RootComponent`) "None" (0.0 0.0 0.0) (struct) "KeepRelativeOffset" false 1.0 1.0 0.0 null null))
        (:`else`)))
    (:`then_2`
      (bind _projectilemuzzlefx (`self.ProjectileMuzzleFX`)
        (:`then`
          (`NiagaraFunctionLibrary.SpawnSystemAtLocation` _projectilemuzzlefx (`self.K2_GetActorLocation`) (`KismetMathLibrary.Conv_VectorToRotator` (`self.GetActorForwardVector`))))
        (:`else`)))))

(event `self.BP_OnSpawnProjectileHitFX`
  (params (HitLocation :type "Vector Structure (by ref)"))
  (`|ExecutionSequence`
    (:`then_0`
      (bind _impactsound (`self.ImpactSound`)
        (:`then`
          (`GameplayStatics.PlaySoundAtLocation` _impactsound HitLocation (struct) 1.0 1.0 0.0 null null null null))
        (:`else`)))
    (:`then_1`
      (bind _impactvfx (`self.ImpactVFX`)
        (:`then`
          (`NiagaraFunctionLibrary.SpawnSystemAtLocation` _impactvfx HitLocation))
        (:`else`)))))

(fn `UserConstructionScript`)